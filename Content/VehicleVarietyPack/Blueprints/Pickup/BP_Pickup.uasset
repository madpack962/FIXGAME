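; BP_Pickup is a drivable pickup vehicle that passes throttle, steering, handbrake and camera input to movement and controller.
; Interaction range toggles a widget, and interacting calls EnterVehicle, which possesses the truck and attaches the passenger to the driver socket; its interface check is disconnected.
; ExitVehicle offsets, detaches and repossesses the passenger, but nothing here calls it.
; Tick feeds absolute forward speed into the engine sound's RPM parameter.
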(event EventTick
  (params (DeltaSeconds :type Float%20%28single-precision%29))
  ;[1 1 1] Звук двигателя
  (Audio|Parameter|SetFloatParameter (Variables|Default|GetEngineSound) "RPM" (Math|Float|Absolute(Float) (Class|WheeledVehicleMovementComponent|GetForwardSpeed (Variables|Default|GetVehicleMovement))) :!class /Script/Engine.AudioComponent))

(event EventOnInteractionRangeEntered
  (Rendering|SetVisibility (Variables|Default|GetWidget) true false))

(event EventOnInteractionRangeExited
  (Rendering|SetVisibility (Variables|Default|GetWidget) false false))

(event EventOnInteracted
  (params (Interactor :type Pawn%20Object%20Reference))
  (CallFunction|EnterVehicle Interactor))

(event Input|ActionEvents|InputActionHandbrake
  (params (Key :type Key%20Structure :default "None"))
  (bind _vehiclemovement (Variables|Default|GetVehicleMovement))
  ;[1 1 1] Управление
  (:Pressed
    (Class|WheeledVehicleMovementComponent|SetHandbrakeInput _vehiclemovement true))
  (:Released
    (Class|WheeledVehicleMovementComponent|SetHandbrakeInput _vehiclemovement false)))

(event Input|ActionEvents|InputActionInteractCar
  (params (Key :type Key%20Structure :default "None")))

(event Input|AxisEvents|InputAxisMoveForward
  (params (AxisValue :type Float%20%28single-precision%29))
  ;[1 1 1] Управление
  (Class|WheeledVehicleMovementComponent|SetThrottleInput (Variables|Default|GetVehicleMovement) AxisValue))

(event Input|AxisEvents|InputAxisMoveRight
  (params (AxisValue :type Float%20%28single-precision%29))
  ;[1 1 1] Управление
  (Class|WheeledVehicleMovementComponent|SetSteeringInput (Variables|Default|GetVehicleMovement) AxisValue))

(event Input|AxisEvents|InputAxisLookUp
  (params (AxisValue :type Float%20%28single-precision%29))
  ;[1 1 1] Управление
  (Pawn|Input|AddControllerPitchInput (* AxisValue -1.0)))

(event Input|AxisEvents|InputAxisLookRight
  (params (AxisValue :type Float%20%28single-precision%29))
  ;[1 1 1] Управление
  (Pawn|Input|AddControllerYawInput AxisValue))

(event Input|AxisEvents|InputAxisLookUp
  (params (AxisValue :type Float%20%28single-precision%29))
  ;[1 1 1] Поворот камеры
  (Pawn|Input|AddControllerPitchInput AxisValue))

(event Input|AxisEvents|InputAxisTurn
  (params (AxisValue :type Float%20%28single-precision%29))
  ;[1 1 1] Поворот камеры
  (Pawn|Input|AddControllerYawInput AxisValue))

(fn ConstructionScript)

(fn EnterVehicle
  (params (Passenger :type Pawn%20Object%20Reference))
  (bind _output_get (Variables|Default|SetPassenger Passenger))
  (Pawn|Possess (Pawn|GetController _output_get) self)
  (Class|PassengerInterface|OnEnterVehicle(Message) (Variables|Default|GetPassenger))
  (Transformation|AttachComponentToComponent (Variables|Default|GetPassenger) (Variables|Character|GetMesh) "DriversSoket" "SnapToTarget" "SnapToTarget" "SnapToTarget" true))

(fn ExitVehicle
  (Transformation|AddActorLocalOffset (Variables|Default|GetPassenger) "0,-150.000000, 0" false true)
  (Transformation|DetachFromActor (Variables|Default|GetPassenger) "KeepWorld" "KeepWorld" "KeepWorld")
  (Class|PassengerInterface|OnExitVehicle(Message) (Variables|Default|GetPassenger))
  (Pawn|Possess (Game|GetPlayerController 0) (Variables|Default|GetPassenger))
  (Variables|Default|SetPassenger 0))